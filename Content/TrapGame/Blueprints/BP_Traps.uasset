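; BP_Traps is a spike trap that moves its spikes up and down continuously and notifies actors that touch it.
; A Timeline started on BeginPlay sets the spike mesh's relative Z from its curve value scaled by PositionLength, then replays in the opposite direction on finish.
; Trigger_Box overlap sends TouchTrapMessage to the overlapping actor and prints that actor's name.
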(event `self.ReceiveBeginPlay`
  (bind (_direction _positionvalue) (`Timeline|Timeline` :!label _label)
    (:`Update`
      (`SceneComponent.K2_SetRelativeLocation` (`self.SM_Spikes`) (`KismetMathLibrary.MakeVector` 0.0 0.0 (* _positionvalue (* (`self.PositionLength`) -1.0))) false false))
    (:`Finished`
      (if (`|EnumEquality` _direction "Forward")
        (`self.Play Backwards`)
        (else
          (`self.Play Forward`))))))

(event `Play Forward`
  (goto _label :!via `PlayFromStart`))

(event `Play Backwards`
  (goto _label :!via `ReverseFromEnd`))

(event `self.Trigger_Box.OnComponentBeginOverlap`
  (params (OverlappedComponent :type "PrimitiveComponent Object Reference") (OtherActor :type "Actor Object Reference") (OtherComp :type "PrimitiveComponent Object Reference") (OtherBodyIndex :type Integer) (bFromSweep :type Boolean) (SweepResult :type "HitResult Structure (by ref)"))
  (message `/Game/TrapGame/Blueprints/BPI_Traps.Touch Trap` OtherActor)
  (`KismetSystemLibrary.PrintString` (`KismetSystemLibrary.GetDisplayName` OtherActor)))

(fn `UserConstructionScript`)